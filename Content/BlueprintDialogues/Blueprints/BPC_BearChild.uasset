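; BPC_BearChild is a dialogue Blueprint for the bear child character that chooses which branch its conversation starts on.
; Every Tick it sets InitialBranch from VisitCount, using a fixed cave branch at zero visits.
; At one visit, the branch depends on the player character's teddy bear flag, and other counts leave it unchanged.
; GetScriptInterpreter supplies the script interpreter held by ThirdPersonGameMode.
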(event EventTick
  (params (DeltaSeconds :type Float%20%28single-precision%29))
  (switch int (Variables|Default|GetVisitCount)
    (:0
      (Variables|Default|SetInitialBranch "Cave1"))
    (:1
      (bind _asthird_person_character (Utilities|Casting|CastToThirdPersonCharacter (Game|GetPlayerCharacter 0)))
      (if (Variables|/Game/ThirdPersonBP/Blueprints/ThirdPersonCharacter.ThirdPersonCharacter_C|GetHas%20TeddyBaer??? _asthird_person_character)
        (Variables|Default|SetInitialBranch "Cave3")
        (else
          (Variables|Default|SetInitialBranch "Cave19"))))))

(fn GetScriptInterpreter
  (return (Variables|/Game/ThirdPersonBP/Blueprints/Audio/ThirdPersonGameMode.ThirdPersonGameMode_C|GetScriptInterp (.AsThird%20Person%20Game%20Mode (Utilities|Casting|CastToThirdPersonGameMode (Game|GetGameMode))))))