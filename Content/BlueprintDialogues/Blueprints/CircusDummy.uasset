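; CircusDummy is a dialogue trigger Blueprint exposing custom events for cave auto-dialogue, tips and a bear moment.
; Each event sends UseMessage with player controller 0 to either the BPCStarlight or BPCTooltips component.
; All but CaveAuto first set BPCStarlight's InitialBranch to a cave branch.
; CaveTip1 and CaveTip3 set that branch on BPCStarlight yet trigger BPCTooltips, whereas the other events trigger BPCStarlight.
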(event Custom|CaveAuto
  (Class|BPIUsable|Use(Message) (Variables|Default|GetBPC_Starlight) (Game|GetPlayerController 0)))

(event Custom|CaveTip1
  (Variables|/Game/BlueprintDialogues/Blueprints/BPC_Dialogue.BPC_Dialogue_C|SetInitialBranch (Variables|Default|GetBPC_Starlight) "Cave14")
  (Class|BPIUsable|Use(Message) (Variables|Default|GetBPC_Tooltips) (Game|GetPlayerController 0)))

(event Custom|CaveTip2
  (bind _bpc_starlight (Variables|Default|GetBPC_Starlight))
  (Variables|/Game/BlueprintDialogues/Blueprints/BPC_Dialogue.BPC_Dialogue_C|SetInitialBranch _bpc_starlight "Cave11")
  (Class|BPIUsable|Use(Message) _bpc_starlight (Game|GetPlayerController 0)))

(event Custom|CaveTip3
  (Variables|/Game/BlueprintDialogues/Blueprints/BPC_Dialogue.BPC_Dialogue_C|SetInitialBranch (Variables|Default|GetBPC_Starlight) "Cave15")
  (Class|BPIUsable|Use(Message) (Variables|Default|GetBPC_Tooltips) (Game|GetPlayerController 0)))

(event Custom|CaveBear
  (bind _bpc_starlight (Variables|Default|GetBPC_Starlight))
  (Variables|/Game/BlueprintDialogues/Blueprints/BPC_Dialogue.BPC_Dialogue_C|SetInitialBranch _bpc_starlight "Cave12")
  (Class|BPIUsable|Use(Message) _bpc_starlight (Game|GetPlayerController 0)))

(fn ConstructionScript)